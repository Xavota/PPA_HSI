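; Terrain actor whose GenerateTerrain function builds a flat, tiled procedural mesh grid; nothing in this Blueprint's live graphs calls it.
; It clears old geometry except normals, then creates vertices, tiled UVs, up-facing normals and grid triangles from Size and Tiles.
; A dynamic material receives the color map and MaxHeight as HeightMult, leaving any displacement to the material.
; The height map and tangent calculation are disconnected.
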(event EventBeginPlay)

(event Collision|EventActorBeginOverlap
  (params (OtherActor :type Actor%20Object%20Reference)))

(event EventTick
  (params (DeltaSeconds :type Float%20%28single-precision%29)))

(fn ConstructionScript)

(fn SetSize
  (params (NewParam :type Vector%202D%20Structure))
  (Variables|Default|SetSize NewParam))

(fn GenerateTerrain
  (params (Size :type Vector%202D%20Structure) (Tiles :type Vector%202D%20Structure) (TextureTiles :type Vector%202D%20Structure) (Material :type Material%20Object%20Reference) (ColorMap :type Texture%20Object%20Reference) (HeightMap :type Texture%20Object%20Reference) (Max%20Height :type Float%20%28single-precision%29))
  (bind (_x _y) (Math|Vector2D|BreakVector2D Size))
  (bind (_x_2 _y_2) (Math|Vector2D|BreakVector2D TextureTiles))
  (bind (_x_3 _y_3) (Math|Vector2D|BreakVector2D Tiles))
  (bind (_x_4 _y_4) (Math|Vector2D|BreakVector2D Tiles))
  (CallFunction|CleanGeometry)
  (Utilities|FlowControl|Sequence
    (:then_0
      (for _index (range 0 (Math|Float|Truncate _x_3))
        (for _index_2 (range 0 (Math|Float|Truncate _y_3))
          (Utilities|Array|Add (Variables|Default|GetVertices) (Math|Vector|MakeVector (* _index (/ _x _x_3)) (* _index_2 (/ _y _y_3)) 0.0))
          (Utilities|Array|Add (Variables|Default|GetUVs) (Math|Vector2D|MakeVector2D (* _x_2 (/ (* _index (/ _x _x_3)) _x)) (* _y_2 (/ (* _index_2 (/ _y _y_3)) _y))))
          (Utilities|Array|Add (Variables|Default|GetNormals) (Math|Vector|MakeVector 0.0 0.0 1.0)))))
    (:then_1
      (bind _triangles (Class|KismetProceduralMeshLibrary|CreateGridMeshTriangles (+ (Math|Float|Truncate _x_4) 1) (+ (Math|Float|Truncate _y_4) 1) false))
      (Variables|Default|SetIndices _triangles)
      (Class|ProceduralMeshComponent|CreateMeshSectionLinearColor (Variables|Default|GetProceduralMesh) 0 (Variables|Default|GetVertices) (Variables|Default|GetIndices) (Variables|Default|GetNormals) (Variables|Default|GetUVs) 0 0 0 0 0 false))
    (:then_2
      (bind _returnvalue (Rendering|Material|CreateDynamicMaterialInstance Material "None" "None" :!class /Script/Engine.KismetMaterialLibrary))
      (Variables|Default|SetDynamicMat _returnvalue)
      (Rendering|Material|SetTextureParameterValue (Variables|Default|GetDynamicMat) "input" ColorMap)
      (Rendering|Material|SetScalarParameterValue (Variables|Default|GetDynamicMat) "HeightMult" Max%20Height :!class /Script/Engine.MaterialInstanceDynamic)
      (Rendering|Material|SetMaterial (Variables|Default|GetProceduralMesh) 0 (Variables|Default|GetDynamicMat)))))

(fn CleanGeometry
  (Utilities|Array|Clear (Variables|Default|GetVertices))
  (Utilities|Array|Clear (Variables|Default|GetUVs))
  (Utilities|Array|Clear (Variables|Default|GetIndices)))